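; Base enemy actor, apparently a mushroom, that emits threat and can be grabbed or destroyed.
; On BeginPlay it takes sounds and attenuation from BP_GameInstance, then after a short delay seeds EnemyThreatComponent with random threat-on-spawn and per-second values and plays its spawn sound.
; Threat changes are relayed through its own dispatcher.
; Grab plays a pickup sound; Destroy broadcasts self-destruct, plays a sound at its location, unbinds listeners and removes the actor.
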(event `self.ReceiveBeginPlay`
  ;[1 1 1] Initialise
  (`self.SetReferences`)
  (`self.BindToComponentEvents`)
  (`self.SetEnemyAudioSFX`)
  (`KismetSystemLibrary.Delay` 0.2)
  (`self.Initialise`)
  (`self.PlaySpawnSFX`))

(event `/Game/Interfaces/BPI_Grabbable.Grab`
  ;[1 1 1] Grab
  (`self.PlayPickUpSFX`))

(event `/Game/Interfaces/BPI_Destructible.Destroy`
  ;[1 1 1] Self Destruct
  (`self.SelfDestruct`))

(fn `BindToComponentEvents`
  ;[1 1 1] Bind to Component Events
  (add `/Game/Components/BP_EnemyThreatComponent.ThreatChanged` (`self.EnemyThreatComponent`) (`|CreateDelegate` :!event `OnThreatChanged`)))

(fn `Initialise`
  (bind _gameinstance (`self.GameInstance`))
  ;[1 1 1] Initialise
  (`/Game/Components/BP_EnemyThreatComponent.Initialise` (`self.EnemyThreatComponent`) (`KismetMathLibrary.RandomFloatInRange` (`/Game/Blueprint/BP_GameInstance.MinimumMushroomThreatEmittedOnSpawn` _gameinstance) (`/Game/Blueprint/BP_GameInstance.MaximumMushroomThreatEmittedOnSpawn` _gameinstance)) (`KismetMathLibrary.RandomFloatInRange` (`/Game/Blueprint/BP_GameInstance.MinimumMushroomThreatEmittedPerSecond` _gameinstance) (`/Game/Blueprint/BP_GameInstance.MaximumMushroomThreatEmittedPerSecond` _gameinstance))))

(fn `OnThreatChanged`
  (params (Value :type "Float (double-precision)"))
  ;[1 1 1] Raise Event
  (`self.ThreatChanged` Value))

(fn `PlayDestroyedSFX`
  ;[1 1 1] Play Destroyed SFX
  (`GameplayStatics.SpawnSoundAtLocation` (`/Game/Blueprint/BP_GameInstance.EnemyDestroyedSFX` (`self.GameInstance`)) (`self.K2_GetActorLocation`) (`self.K2_GetActorRotation`) 1.0 1.0 0.0 (`/Game/Blueprint/BP_GameInstance.EnemyDestroyedAttenuation` (`self.GameInstance`)) null))

(fn `PlayPickUpSFX`
  ;[1 1 1] Play Pick Up SFX
  (if (not (`AudioComponent.IsPlaying` (`self.AudioPickUp`)))
    (`AudioComponent.Play` (`self.AudioPickUp`) 0.0)))

(fn `PlaySpawnSFX`
  ;[1 1 1] Play Spawn SFX
  (if (not (`AudioComponent.IsPlaying` (`self.AudioSpawn`)))
    (`AudioComponent.Play` (`self.AudioSpawn`) 0.0)))

(fn `SelfDestruct`
  ;[1 1 1] Self Destruct
  (`self.SelfDestructInitiated`)
  (`self.PlayDestroyedSFX`)
  (`self.UnbindEvents`)
  (`self.K2_DestroyActor`))

(fn `SetEnemyAudioSFX`
  ;[1 1 1] Set Enemy Audio SFX
  (`AudioComponent.SetSound` (`self.AudioSpawn`) (`/Game/Blueprint/BP_GameInstance.EnemySpawnSFX` (`self.GameInstance`)))
  (set `AudioComponent.AttenuationSettings` (`/Game/Blueprint/BP_GameInstance.EnemySpawnAttenuation` (`self.GameInstance`)) (`self.AudioSpawn`))
  (`AudioComponent.SetSound` (`self.AudioPickUp`) (`/Game/Blueprint/BP_GameInstance.EnemyPickUpSFX` (`self.GameInstance`)))
  (set `AudioComponent.AttenuationSettings` (`/Game/Blueprint/BP_GameInstance.EnemyPickUpAttenuation` (`self.GameInstance`)) (`self.AudioPickUp`)))

(fn `SetReferences`
  ;[1 1 1] Set References
  (bind _asbp_game_instance (cast `/Game/Blueprint/BP_GameInstance` (`GameplayStatics.GetGameInstance`)))
  (set `self.GameInstance` _asbp_game_instance))

(fn `UnbindEvents`
  ;[1 1 1] Unbind Events
  (clear `self.ThreatChanged`)
  (clear `self.SelfDestructInitiated`))

(fn `UserConstructionScript`)