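; Game state Blueprint that keeps a running Threat total fed by enemies from the level's spawners.
; On BeginPlay, a looping timer polls HasBegunPlay, then clears itself, caches all BP_EnemySpawner actors and binds to their spawn events.
; Each spawned enemy gets its threat-changed event bound, and the handler adds the reported value to Threat.
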(event `self.ReceiveBeginPlay`
  ;[1 1 1] Initialise
  (bind _returnvalue (`KismetSystemLibrary.K2_SetTimer` null "CanSetReferences" 0.1 true))
  (set `self.HasBegunPlayTimer` _returnvalue))

(fn `BindToEvents`
  ;[1 1 1] Bind to Events
  (for _array_element (`self.EnemySpawners`)
    (add `/Game/Blueprint/BP_EnemySpawner.EnemySpawned` _array_element (`|CreateDelegate` :!event `OnEnemySpawned`))))

(fn `CanSetReferences`
  ;[1 1 1] Can Set References?
  (if (`self.HasBegunPlay`)
    (`KismetSystemLibrary.K2_ClearAndInvalidateTimerHandle` (`self.HasBegunPlayTimer`))
    (`self.SetReferences`)
    (`self.BindToEvents`)))

(fn `OnEnemySpawned`
  (params (Enemy :type "/Game/Blueprint/BP_EnemyBase Object Reference"))
  ;[1 1 1] Event Handler
  (add `/Game/Blueprint/BP_EnemyBase.ThreatChanged` Enemy (`|CreateDelegate` :!event `OnEnemyThreatChanged`)))

(fn `OnEnemyThreatChanged`
  (params (Value :type "Float (double-precision)"))
  ;[1 1 1] Event Handler
  (set `self.Threat` (+ (`self.Threat`) Value)))

(fn `SetReferences`
  ;[1 1 1] Set References
  (bind _outactors (`GameplayStatics.GetAllActorsOfClass` "/Game/Blueprint/BP_EnemySpawner.BP_EnemySpawner_C"))
  (set `self.EnemySpawners` _outactors))

(fn `UserConstructionScript`)