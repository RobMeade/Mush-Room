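; Spawner actor that periodically places BP_Mushroom enemies on surfaces below a configurable box volume and announces each spawn.
; A looping timer uses an initial random delay from the GameInstance; later re-rolls never reset it.
; Each spawn line-traces down from a random point and aligns the mushroom to the surface normal.
; CanSpawn updates against the GameInstance cap only after spawning, not when enemies self-destruct, and game over clears it.
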(event `self.ReceiveBeginPlay`
  ;[1 1 1] Initialise
  (`self.SetReferences`)
  (`self.BindToEvents`)
  (`self.SetRandomSpawnDelay`)
  (`KismetSystemLibrary.K2_SetTimerDelegate` (`|CreateDelegate` :!event `OnSpawn`) (`self._SpawnDelay`) true (`self._SpawnDelay`)))

(fn `BindToEvents`
  ;[1 1 1] Bind to Events
  (add `/Game/Blueprint/BP_GameMode.GameOverInitiated` (`self._GameMode`) (`|CreateDelegate` :!event `OnGameOverInitiated`)))

(fn `GetRandomSpawnLocation`
  (returns (SpawnLocation :type "Vector Structure"))
  (bind (_returnvalue_x _returnvalue_y _returnvalue_z) (`KismetMathLibrary.BreakVector` (`self.K2_GetActorLocation`)))
  (bind _spawnvolume (`self.SpawnVolume`))
  ;[1 1 1] Get Random Spawn Location
  (return (`KismetMathLibrary.MakeVector` (.x (+ (`self.K2_GetActorLocation`) (`KismetMathLibrary.RandomPointInBoundingBox` (`SceneComponent.RelativeLocation` _spawnvolume) (`BoxComponent.BoxExtent` _spawnvolume)))) (.y (+ (`self.K2_GetActorLocation`) (`KismetMathLibrary.RandomPointInBoundingBox` (`SceneComponent.RelativeLocation` _spawnvolume) (`BoxComponent.BoxExtent` _spawnvolume)))) (+ _returnvalue_z (`self.SpawnVolumeHeight`)))))

(fn `IsSpawnLocationValid`
  (params (SpawnLocation :type "Vector Structure"))
  (returns (Result :type Boolean))
  ;[1 1 1] Is Spawn Location Valid
  (bind _outhit (`KismetSystemLibrary.LineTraceSingle` SpawnLocation (`KismetMathLibrary.MakeVector` (.x SpawnLocation) (.y SpawnLocation) (* (.z SpawnLocation) -1.0)) "TraceTypeQuery1" true))
  (bind (_bblockinghit _binitialoverlap _time _distance _location _impactpoint _normal _impactnormal) (`GameplayStatics.BreakHitResult` _outhit))
  (if _bblockinghit
    (set `self._SpawnTransform` (`KismetMathLibrary.MakeTransform` _impactpoint (`KismetMathLibrary.MakeRotFromZX` _impactnormal (`SceneComponent.GetForwardVector` (`self.DefaultSceneRoot`)))))
    (return true)
    (else
      (return false))))

(fn `OnEnemyDestroyed`
  ;[1 1 1] Event Handler
  (`/Engine/EditorBlueprintResources/StandardMacros.DecrementInt` (`self._SpawnedEnemies`)))

(fn `OnGameOverInitiated`
  (params (Outcome :type "/Game/Enum/EGameOverOutcome Enum" :default "NewEnumerator0"))
  ;[1 1 1] Event Handler
  (set `self._CanSpawn` false))

(fn `OnSpawn`
  ;[1 1 1] Event Handler
  (`self.SetRandomSpawnDelay`)
  (if (`self._CanSpawn`)
    (`self.Spawn`)))

(fn `SetCanSpawn`
  ;[1 1 1] Set Can Spawn
  (set `self._CanSpawn` (< (`self._SpawnedEnemies`) (`/Game/Blueprint/BP_GameInstance.MaximumMushroomSpawnCount` (`self._GameInstance`)))))

(fn `SetRandomSpawnDelay`
  (bind __gameinstance (`self._GameInstance`))
  ;[1 1 1] Set Random Spawn Delay
  (set `self._SpawnDelay` (`KismetMathLibrary.RandomFloatInRange` (`/Game/Blueprint/BP_GameInstance.MinimumMushroomSpawnDelay` __gameinstance) (`/Game/Blueprint/BP_GameInstance.MaximumMushroomSpawnDelay` __gameinstance))))

(fn `SetReferences`
  ;[1 1 1] Set References
  (bind _asbp_game_instance (cast `/Game/Blueprint/BP_GameInstance` (`GameplayStatics.GetGameInstance`)))
  (set `self._GameInstance` _asbp_game_instance)
  (bind _asbp_game_mode (cast `/Game/Blueprint/BP_GameMode` (`GameplayStatics.GetGameMode`)))
  (set `self._GameMode` _asbp_game_mode))

(fn `Spawn`
  (locals (SpawnedEnemy :type "/Game/Blueprint/BP_EnemyBase Object Reference"))
  ;[1 1 1] Spawn
  (bind _spawnlocation (`self.GetRandomSpawnLocation`))
  (bind _result (`self.IsSpawnLocationValid` _spawnlocation))
  (if _result
    (bind _returnvalue (`|SpawnActorFromClass` "/Game/Blueprint/BP_Mushroom.BP_Mushroom_C" (`self._SpawnTransform`) "Undefined" "OverrideRootScale" null null))
    (set `local.SpawnedEnemy` _returnvalue)
    (`/Engine/EditorBlueprintResources/StandardMacros.IncrementInt` (`self._SpawnedEnemies`)
      (:`  `
        (`self.SetCanSpawn`)
        (add `/Game/Blueprint/BP_EnemyBase.SelfDestructInitiated` (`local.SpawnedEnemy`) (`|CreateDelegate` :!event `OnEnemyDestroyed`))
        (`self.EnemySpawned` (`local.SpawnedEnemy`))))))

(fn `UserConstructionScript`
  (bind _returnvalue (/ (`self.SpawnVolumeHeight`) 2.0))
  (`BoxComponent.SetBoxExtent` (`self.SpawnVolume`) (`KismetMathLibrary.MakeVector` (/ (`self.SpawnVolumeWidth`) 2.0) (/ (`self.SpawnVolumeLength`) 2.0) _returnvalue) true)
  (`SceneComponent.K2_SetRelativeLocation` (`self.SpawnVolume`) (`KismetMathLibrary.MakeVector` 0.0 0.0 _returnvalue) false false))