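; Cauldron prop that plays a sound and sends a destroy message to any overlapping actor implementing BPI_Destructible.
; On BeginPlay it caches BP_GameInstance, binds to player preference changes and pulls its sound and attenuation from the game instance.
; The entry sound never restarts while playing.
; Its volume follows SFX mute and volume preferences, substituting a minimum safe multiplier for near-zero values.
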(event `self.ReceiveBeginPlay`
  ;[1 1 1] Initialise
  (`self.SetReferences`)
  (`self.BindToEvents`)
  (`self.SetCauldronAudioSFX`))

(event `self.Collision.OnComponentBeginOverlap`
  (params (OverlappedComponent :type "PrimitiveComponent Object Reference") (OtherActor :type "Actor Object Reference") (OtherComp :type "PrimitiveComponent Object Reference") (OtherBodyIndex :type Integer) (bFromSweep :type Boolean) (SweepResult :type "HitResult Structure (by ref)"))
  ;[1 1 1] On Overlap
  (`self.PlayCauldronObjectEnteredSFX`)
  (if (`KismetSystemLibrary.DoesImplementInterface` OtherActor "/Game/Interfaces/BPI_Destructible.BPI_Destructible_C")
    (message `/Game/Interfaces/BPI_Destructible.Destroy` OtherActor)))

(fn `BindToEvents`
  ;[1 1 1] Bind to Events
  (add `/Game/Blueprint/BP_GameInstance.PlayerPreferencesChanged` (`self._GameInstance`) (`|CreateDelegate` :!event `OnPlayerPreferencesChanged`)))

(fn `GetSafeVolumeMultiplier`
  (params (Volume :type "Float (double-precision)"))
  (returns (SafeVolumeMultiplier :type "Float (double-precision)"))
  ;[1 1 1] Get Safe Volume Multiplier
  (if (`KismetMathLibrary.NearlyEqual_FloatFloat` Volume)
    (return (`/Game/Blueprint/BP_GameInstance.MinimumSafeVolumeMultiplier` (`self._GameInstance`)))
    (else
      (return (`local.Volume`)))))

(fn `OnPlayerPreferencesChanged`
  ;[1 1 1] Player Preferences Changed
  (`self.SetCauldronAudioVolumeMultiplier`))

(fn `PlayCauldronObjectEnteredSFX`
  ;[1 1 1] Play Cauldron Object Entered SFX
  (if (not (`AudioComponent.IsPlaying` (`self.AudioObjectEntered`)))
    (`AudioComponent.Play` (`self.AudioObjectEntered`) 0.0)))

(fn `SetCauldronAudioSFX`
  ;[1 1 1] Set Cauldron Audio SFX
  (`AudioComponent.SetSound` (`self.AudioObjectEntered`) (`/Game/Blueprint/BP_GameInstance.CauldronObjectEnteredSFX` (`self._GameInstance`)))
  (set `AudioComponent.AttenuationSettings` (`/Game/Blueprint/BP_GameInstance.CauldronObjectEnteredAttenuation` (`self._GameInstance`)) (`self.AudioObjectEntered`))
  (`self.SetCauldronAudioVolumeMultiplier`))

(fn `SetCauldronAudioVolumeMultiplier`
  (bind _playerpreferences (`/Game/Blueprint/BP_GameInstance.PlayerPreferences` (`self._GameInstance`)))
  ;[1 1 1] Set Cauldron Audio Volume Multiplier
  (`AudioComponent.SetVolumeMultiplier` (`self.AudioObjectEntered`) (`self.GetSafeVolumeMultiplier` (select `bool` (`.SFXIsMuted_9_E23DD18040ECD7EB8BF0C2ADB75E2B00` (break `/Game/Structures/SPlayerPreferencesAudio` (break `/Game/Structures/SPlayerPreferences` _playerpreferences))) :`false` (`.SFXVolume_4_5A5A80D44E041048BB7E85A513693288` (break `/Game/Structures/SPlayerPreferencesAudio` (break `/Game/Structures/SPlayerPreferences` _playerpreferences)))))))

(fn `SetReferences`
  ;[1 1 1] Set References
  (bind _asbp_game_instance (cast `/Game/Blueprint/BP_GameInstance` (`GameplayStatics.GetGameInstance`)))
  (set `self._GameInstance` _asbp_game_instance))

(fn `UserConstructionScript`)