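; Save game object that persists the player's preferences to a named slot.
; Initialise sets the preferences in memory only, while SaveData sets them and writes the object to the slot.
; LoadData copies preferences from an existing save into itself and returns them, or writes itself to create the slot when none exists and returns its current values.
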(fn `Initialise`
  (params (PlayerPreferences :type "/Game/Core/Structures/PlayerPreferences/SPlayerPreferences Structure"))
  ;[1 1 1] Initialise
  (set `self.PlayerPreferences` PlayerPreferences))

(fn `LoadData`
  (returns (PlayerPreferences :type "/Game/Core/Structures/PlayerPreferences/SPlayerPreferences Structure"))
  ;[1 1 1] Load Data
  (bind _returnvalue (`GameplayStatics.DoesSaveGameExist` (`self.SlotName`)))
  (if _returnvalue
    (bind _returnvalue_2 (`GameplayStatics.LoadGameFromSlot` (`self.SlotName`)))
    (bind _asbp_save_game (cast `/Game/Core/BP_SaveGame` _returnvalue_2))
    (set `self.PlayerPreferences` (`/Game/Core/BP_SaveGame.PlayerPreferences` _asbp_save_game))
    (else
      (`GameplayStatics.SaveGameToSlot` self (`self.SlotName`))))
  (return (`self.PlayerPreferences`)))

(fn `SaveData`
  (params (PlayerPreferences :type "/Game/Core/Structures/PlayerPreferences/SPlayerPreferences Structure"))
  ;[1 1 1] Save Data
  (set `self.PlayerPreferences` PlayerPreferences)
  (`GameplayStatics.SaveGameToSlot` self (`self.SlotName`)))