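; Gameplay game mode that ends the game on threat limits, controls pausing and plays in-game music.
; On BeginPlay it caches the game instance, game state and player controller, then binds to their threat, initialisation, pause and volume events.
; Threat reaching either threshold broadcasts a game-over outcome, and pause toggles are broadcast too.
; Music follows player preferences, with zero or muted volume replaced by a minimum safe multiplier.
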(event `self.ReceiveBeginPlay`
  ;[1 1 1] Initialise
  (`self.SetReferences`)
  (`self.BindToEvents`)
  (`self.PlayMusic`))

(fn `BindToEvents`
  ;[1 1 1] Bind to Events
  (add `/Game/Core/BP_GameState.ThreatChanged` (`self._GameState`) (`|CreateDelegate` :!event `OnThreatChanged`))
  (add `/Game/Core/Characters/Player/BP_PlayerController.PlayerControllerInitialised` (`self._PlayerController`) (`|CreateDelegate` :!event `OnPlayerControllerInitialised`))
  (add `/Game/Core/Characters/Player/BP_PlayerController.PlayerPauseGameToggled` (`self._PlayerController`) (`|CreateDelegate` :!event `OnPlayerPauseGameToggled`))
  (add `/Game/Core/Characters/Player/BP_PlayerController.MusicVolumeControlChanged` (`self._PlayerController`) (`|CreateDelegate` :!event `OnMusicVolumeControlChanged`)))

(fn `GameOver`
  (params (Outcome :type "/Game/Core/Enums/EGameOverOutcome Enum" :default "NewEnumerator0"))
  ;[1 1 1] Game Over
  (`self.GameOverInitiated` Outcome))

(fn `GetSafeVolumeMultiplier`
  (params (Volume :type "Float (double-precision)"))
  (returns (SafeVolumeMultiplier :type "Float (double-precision)"))
  ;[1 1 1] Get Safe Volume Multiplier
  (if (`KismetMathLibrary.NearlyEqual_FloatFloat` Volume)
    (return (`/Game/Core/BP_GameInstance.MinimumSafeVolumeMultiplier` (`self._GameInstance`)))
    (else
      (return (`local.Volume`)))))

(fn `OnMusicVolumeControlChanged`
  (params (Volume :type "Float (double-precision)") (IsMuted :type Boolean))
  ;[1 1 1] Music Volume Control Changed
  (`AudioComponent.SetVolumeMultiplier` (`self.AudioMusic`) (`self.GetSafeVolumeMultiplier` (select `bool` IsMuted :`false` Volume))))

(fn `OnPlayerControllerInitialised`
  ;[1 1 1] Player Controller Initialised
  (`/Game/Core/Characters/Player/BP_PlayerController.InitialiseForGame` (`self._PlayerController`)))

(fn `OnPlayerPauseGameToggled`
  ;[1 1 1] Player Pause Game Toggled
  (`self.TogglePauseGame`))

(fn `OnThreatChanged`
  (params (Value :type "Float (double-precision)"))
  ;[1 1 1] Event Handler
  (if (>= Value (`/Game/Core/BP_GameInstance.MaximumThreatThreshold` (`self._GameInstance`)))
    (`self.GameOver` "NewEnumerator1")
    (elif (<= Value (`/Game/Core/BP_GameInstance.MinimumThreatThreshold` (`self._GameInstance`)))
      (`self.GameOver` "NewEnumerator0"))))

(fn `PlayMusic`
  (bind _playerpreferences (`/Game/Core/BP_GameInstance.PlayerPreferences` (`self._GameInstance`)))
  ;[1 1 1] Play Music
  (`AudioComponent.SetVolumeMultiplier` (`self.AudioMusic`) (`self.GetSafeVolumeMultiplier` (select `bool` (`.MusicIsMuted_7_D39A27A54CA7C605BDDFC6B0407D0135` (break `/Game/Core/Structures/PlayerPreferences/SPlayerPreferencesAudio` (break `/Game/Core/Structures/PlayerPreferences/SPlayerPreferences` _playerpreferences))) :`false` (break `/Game/Core/Structures/PlayerPreferences/SPlayerPreferencesAudio` (break `/Game/Core/Structures/PlayerPreferences/SPlayerPreferences` _playerpreferences)))))
  (`AudioComponent.SetSound` (`self.AudioMusic`) (`/Game/Core/BP_GameInstance.MusicGame` (`self._GameInstance`)))
  (`AudioComponent.Play` (`self.AudioMusic`) 0.0))

(fn `SetReferences`
  ;[1 1 1] Set References
  (bind _asbp_game_instance (cast `/Game/Core/BP_GameInstance` (`GameplayStatics.GetGameInstance`)))
  (set `self._GameInstance` _asbp_game_instance)
  (bind _asbp_game_state (cast `/Game/Core/BP_GameState` (`GameplayStatics.GetGameState`)))
  (set `self._GameState` _asbp_game_state)
  (bind _asbp_player_controller (cast `/Game/Core/Characters/Player/BP_PlayerController` (`GameplayStatics.GetPlayerController` 0)))
  (set `self._PlayerController` _asbp_player_controller))

(fn `TogglePauseGame`
  (bind _returnvalue (`GameplayStatics.IsGamePaused`))
  ;[1 1 1] Toggle Pause Game
  (`GameplayStatics.SetGamePaused` (select `bool` _returnvalue :`false` true))
  (`self.GamePauseToggled` _returnvalue))

(fn `UserConstructionScript`)