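; Base NPC enemy that emits threat, plays spawn, pickup and destroyed sounds, and can self-destruct.
; After a short BeginPlay delay, it seeds EnemyThreatComponent with random GameInstance mushroom threat rates and re-broadcasts threat changes.
; GameMode game over stops threat emission, while preference changes update SFX volume, substituting a safe minimum for zero.
; Self-destruct broadcasts, spawns a detached sound, clears its own dispatchers, then destroys the actor.
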(event `self.ReceiveBeginPlay`
  ;[1 1 1] Initialise
  (`self.SetReferences`)
  (`self.BindToEvents`)
  (`self.BindToComponentEvents`)
  (`self.SetEnemyAudioSFX`)
  (`KismetSystemLibrary.Delay` 0.2)
  (`self.Initialise`)
  (`self.PlaySpawnSFX`))

(event `/Game/Core/Interfaces/BPI_Grabbable.Grab`
  ;[1 1 1] Grab
  (`self.PlayPickUpSFX`))

(event `/Game/Core/Interfaces/BPI_Destructible.Destroy`
  ;[1 1 1] Self Destruct
  (`self.SelfDestruct`))

(fn `BindToComponentEvents`
  ;[1 1 1] Bind to Component Events
  (add `/Game/Core/Characters/NPC/BP_EnemyThreatComponent.ThreatChanged` (`self.EnemyThreatComponent`) (`|CreateDelegate` :!event `OnThreatChanged`)))

(fn `BindToEvents`
  ;[1 1 1] Bind to Events
  (add `/Game/Core/BP_GameInstance.PlayerPreferencesChanged` (`self._GameInstance`) (`|CreateDelegate` :!event `OnPlayerPreferencesChanged`))
  (add `/Game/Core/GameModes/BP_GameMode.GameOverInitiated` (`self._GameMode`) (`|CreateDelegate` :!event `OnGameOverInitiated`)))

(fn `GetSafeVolumeMultiplier`
  (params (Volume :type "Float (double-precision)"))
  (returns (SafeVolumeMultiplier :type "Float (double-precision)"))
  ;[1 1 1] Get Safe Volume Multiplier
  (if (`KismetMathLibrary.NearlyEqual_FloatFloat` Volume)
    (return (`/Game/Core/BP_GameInstance.MinimumSafeVolumeMultiplier` (`self._GameInstance`)))
    (else
      (return (`local.Volume`)))))

(fn `Initialise`
  (bind __gameinstance (`self._GameInstance`))
  ;[1 1 1] Initialise
  (`/Game/Core/Characters/NPC/BP_EnemyThreatComponent.Initialise` (`self.EnemyThreatComponent`) (`KismetMathLibrary.RandomFloatInRange` (`/Game/Core/BP_GameInstance.MinimumMushroomThreatEmittedOnSpawn` __gameinstance) (`/Game/Core/BP_GameInstance.MaximumMushroomThreatEmittedOnSpawn` __gameinstance)) (`KismetMathLibrary.RandomFloatInRange` (`/Game/Core/BP_GameInstance.MinimumMushroomThreatEmittedPerSecond` __gameinstance) (`/Game/Core/BP_GameInstance.MaximumMushroomThreatEmittedPerSecond` __gameinstance))))

(fn `OnGameOverInitiated`
  (params (Outcome :type "/Game/Core/Enums/EGameOverOutcome Enum" :default "NewEnumerator0"))
  ;[1 1 1] Event Handler
  (`/Game/Core/Characters/NPC/BP_EnemyThreatComponent.StopEmittingThreat` (`self.EnemyThreatComponent`)))

(fn `OnPlayerPreferencesChanged`
  ;[1 1 1] Player Preferences Updated
  (`self.SetEnemyAudioVolumeMultiplier`))

(fn `OnThreatChanged`
  (params (Value :type "Float (double-precision)"))
  ;[1 1 1] Raise Event
  (`self.ThreatChanged` Value))

(fn `PlayDestroyedSFX`
  (bind _playerpreferences (`/Game/Core/BP_GameInstance.PlayerPreferences` (`self._GameInstance`)))
  ;[1 1 1] Play Destroyed SFX
  (`GameplayStatics.SpawnSoundAtLocation` (`/Game/Core/BP_GameInstance.EnemyDestroyedSFX` (`self._GameInstance`)) (`self.K2_GetActorLocation`) (`self.K2_GetActorRotation`) (`self.GetSafeVolumeMultiplier` (select `bool` (`.SFXIsMuted_9_E23DD18040ECD7EB8BF0C2ADB75E2B00` (break `/Game/Core/Structures/PlayerPreferences/SPlayerPreferencesAudio` (break `/Game/Core/Structures/PlayerPreferences/SPlayerPreferences` _playerpreferences))) :`false` (`.SFXVolume_4_5A5A80D44E041048BB7E85A513693288` (break `/Game/Core/Structures/PlayerPreferences/SPlayerPreferencesAudio` (break `/Game/Core/Structures/PlayerPreferences/SPlayerPreferences` _playerpreferences))))) 1.0 0.0 (`/Game/Core/BP_GameInstance.EnemyDestroyedAttenuation` (`self._GameInstance`)) null))

(fn `PlayPickUpSFX`
  ;[1 1 1] Play Pick Up SFX
  (if (not (`AudioComponent.IsPlaying` (`self.AudioPickUp`)))
    (`AudioComponent.Play` (`self.AudioPickUp`) 0.0)))

(fn `PlaySpawnSFX`
  ;[1 1 1] Play Spawn SFX
  (if (not (`AudioComponent.IsPlaying` (`self.AudioSpawn`)))
    (`AudioComponent.Play` (`self.AudioSpawn`) 0.0)))

(fn `SelfDestruct`
  ;[1 1 1] Self Destruct
  (`self.SelfDestructInitiated`)
  (`self.PlayDestroyedSFX`)
  (`self.UnbindEvents`)
  (`self.K2_DestroyActor`))

(fn `SetEnemyAudioSFX`
  ;[1 1 1] Set Enemy Audio SFX
  (`AudioComponent.SetSound` (`self.AudioSpawn`) (`/Game/Core/BP_GameInstance.EnemySpawnSFX` (`self._GameInstance`)))
  (set `AudioComponent.AttenuationSettings` (`/Game/Core/BP_GameInstance.EnemySpawnAttenuation` (`self._GameInstance`)) (`self.AudioSpawn`))
  (`AudioComponent.SetSound` (`self.AudioPickUp`) (`/Game/Core/BP_GameInstance.EnemyPickUpSFX` (`self._GameInstance`)))
  (set `AudioComponent.AttenuationSettings` (`/Game/Core/BP_GameInstance.EnemyPickUpAttenuation` (`self._GameInstance`)) (`self.AudioPickUp`))
  (`self.SetEnemyAudioVolumeMultiplier`))

(fn `SetEnemyAudioVolumeMultiplier`
  (bind _playerpreferences (`/Game/Core/BP_GameInstance.PlayerPreferences` (`self._GameInstance`)))
  (bind _safevolumemultiplier (`self.GetSafeVolumeMultiplier` (select `bool` (`.SFXIsMuted_9_E23DD18040ECD7EB8BF0C2ADB75E2B00` (break `/Game/Core/Structures/PlayerPreferences/SPlayerPreferencesAudio` (break `/Game/Core/Structures/PlayerPreferences/SPlayerPreferences` _playerpreferences))) :`false` (`.SFXVolume_4_5A5A80D44E041048BB7E85A513693288` (break `/Game/Core/Structures/PlayerPreferences/SPlayerPreferencesAudio` (break `/Game/Core/Structures/PlayerPreferences/SPlayerPreferences` _playerpreferences))))))
  ;[1 1 1] Set Enemy Audio Volume Multipler
  (`AudioComponent.SetVolumeMultiplier` (`self.AudioSpawn`) _safevolumemultiplier)
  (`AudioComponent.SetVolumeMultiplier` (`self.AudioPickUp`) _safevolumemultiplier))

(fn `SetReferences`
  ;[1 1 1] Set References
  (bind _asbp_game_instance (cast `/Game/Core/BP_GameInstance` (`GameplayStatics.GetGameInstance`)))
  (set `self._GameInstance` _asbp_game_instance)
  (bind _asbp_game_mode (cast `/Game/Core/GameModes/BP_GameMode` (`GameplayStatics.GetGameMode`)))
  (set `self._GameMode` _asbp_game_mode))

(fn `UnbindEvents`
  ;[1 1 1] Unbind Events
  (clear `self.ThreatChanged`)
  (clear `self.SelfDestructInitiated`))

(fn `UserConstructionScript`)