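; Game mode for the introduction, which plays the menu music and sets up the player controller for that stage.
; On BeginPlay it caches the game instance and player controller, binds to controller initialisation, applies saved audio preferences and disables input.
; Once the controller is initialised, it switches it into introduction setup.
; Music volume handling respects mute and substitutes a minimum safe multiplier for near-zero values.
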(event `self.ReceiveBeginPlay`
  (bind __playercontroller (`self._PlayerController`))
  ;[1 1 1] Initialise
  (`self.SetReferences`)
  (`self.BindToEvents`)
  (`self.ApplyPlayerPreferences`)
  (`self.DisableInput` __playercontroller __playercontroller)
  (`self.PlayMusic`))

(fn `ApplyPlayerPreferences`
  (bind (_audiopreferences_musicvolume _audiopreferences_musicismuted) (break `/Game/ProjectName/Core/Structures/PlayerPreferences/SPlayerPreferencesAudio` (`/Game/ProjectName/Core/BP_GameInstance.GetPlayerPreferencesAudio` (`self._GameInstance`))))
  ;[1 1 1] Apply Player Preferences
  (`AudioComponent.SetVolumeMultiplier` (`self.AudioMusic`) (`self.GetSafeVolumeMultiplier` (select `bool` _audiopreferences_musicismuted :`false` _audiopreferences_musicvolume))))

(fn `BindToEvents`
  ;[1 1 1] Bind to Events
  (add `/Game/ProjectName/Core/Characters/Player/BP_PlayerController.PlayerControllerInitialised` (`self._PlayerController`) (`|CreateDelegate` :!event `OnPlayerControllerInitialised`)))

(fn `GetSafeVolumeMultiplier`
  (params (Volume :type "Float (double-precision)"))
  (returns (SafeVolumeMultiplier :type "Float (double-precision)"))
  ;[1 1 1] Get Safe Volume Multiplier
  (if (`KismetMathLibrary.NearlyEqual_FloatFloat` Volume)
    (return (`/Game/ProjectName/Core/BP_GameInstance.MinimumSafeVolumeMultiplier` (`self._GameInstance`)))
    (else
      (return (`local.Volume`)))))

(fn `OnMusicVolumeChanged`
  (params (Volume :type "Float (double-precision)") (IsMute :type Boolean))
  ;[1 1 1] Music Volume Changed
  (`AudioComponent.SetVolumeMultiplier` (`self.AudioMusic`) (`self.GetSafeVolumeMultiplier` (select `bool` IsMute :`false` Volume))))

(fn `OnPlayerControllerInitialised`
  ;[1 1 1] Player Controller Initialised
  (`/Game/ProjectName/Core/Characters/Player/BP_PlayerController.InitialiseForIntroduction` (`self._PlayerController`)))

(fn `PlayMusic`
  ;[1 1 1] Play Music
  (`AudioComponent.SetSound` (`self.AudioMusic`) (`/Game/ProjectName/Core/BP_GameInstance.MusicMenu` (`self._GameInstance`)))
  (`AudioComponent.Play` (`self.AudioMusic`) 0.0))

(fn `SetReferences`
  ;[1 1 1] Set References
  (bind _asbp_game_instance (cast `/Game/ProjectName/Core/BP_GameInstance` (`GameplayStatics.GetGameInstance`)))
  (set `self._GameInstance` _asbp_game_instance)
  (bind _asbp_player_controller (cast `/Game/ProjectName/Core/Characters/Player/BP_PlayerController` (`GameplayStatics.GetPlayerController` 0)))
  (set `self._PlayerController` _asbp_player_controller))

(fn `UserConstructionScript`)