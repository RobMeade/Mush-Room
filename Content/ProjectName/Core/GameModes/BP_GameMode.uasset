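; Game mode for gameplay levels that ends the match, handles pausing, plays music and applies player audio and brightness preferences.
; On BeginPlay it caches the game instance, game state, player controller and first post-process volume, then binds handlers to their events.
; Active enemies reaching zero or threat hitting its maximum triggers game over and pauses the game.
; Brightness maps to exposure compensation, and near-zero music volume is replaced by a safe minimum multiplier.
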(event `self.ReceiveBeginPlay`
  ;[1 1 1] Initialise
  (`self.SetReferences`)
  (`self.BindToEvents`)
  (`self.ApplyPlayerPreferences`)
  (`self.PlayMusic`))

(fn `ApplyPlayerPreferences`
  (bind (_audiopreferences_musicvolume _audiopreferences_musicismuted) (break `/Game/ProjectName/Core/Structures/PlayerPreferences/SPlayerPreferencesAudio` (`/Game/ProjectName/Core/BP_GameInstance.GetPlayerPreferencesAudio` (`self._GameInstance`))))
  (bind (_graphicspreferences_windowmode _graphicspreferences_screenresolution _graphicspreferences_brightness) (break `/Game/ProjectName/Core/Structures/PlayerPreferences/SPlayerPreferencesGraphics` (`/Game/ProjectName/Core/BP_GameInstance.GetPlayerPreferencesGraphics` (`self._GameInstance`))))
  ;[1 1 1] Apply Player Preferences
  (`AudioComponent.SetVolumeMultiplier` (`self.AudioMusic`) (`self.GetSafeVolumeMultiplier` (select `bool` _audiopreferences_musicismuted :`false` _audiopreferences_musicvolume)))
  (`self.SetBrightness` _graphicspreferences_brightness))

(fn `BindToEvents`
  ;[1 1 1] Bind to Events
  (add `/Game/ProjectName/Core/BP_GameState.ActiveEnemiesChanged` (`self._GameState`) (`|CreateDelegate` :!event `OnActiveEnemiesChanged`))
  (add `/Game/ProjectName/Core/BP_GameState.ThreatChanged` (`self._GameState`) (`|CreateDelegate` :!event `OnThreatChanged`))
  (add `/Game/ProjectName/Core/Characters/Player/BP_PlayerController.PlayerControllerInitialised` (`self._PlayerController`) (`|CreateDelegate` :!event `OnPlayerControllerInitialised`))
  (add `/Game/ProjectName/Core/Characters/Player/BP_PlayerController.PlayerPauseGameToggled` (`self._PlayerController`) (`|CreateDelegate` :!event `OnPlayerPauseGameToggled`))
  (add `/Game/ProjectName/Core/Characters/Player/BP_PlayerController.MusicVolumeControlChanged` (`self._PlayerController`) (`|CreateDelegate` :!event `OnMusicVolumeControlChanged`))
  (add `/Game/ProjectName/Core/Characters/Player/BP_PlayerController.BrightnessValueChanged` (`self._PlayerController`) (`|CreateDelegate` :!event `OnBrightnessValueChanged`)))

(fn `GameOver`
  (params (Outcome :type "/Game/ProjectName/Core/Enums/EGameOverOutcome Enum" :default "NewEnumerator0"))
  ;[1 1 1] Game Over
  (`self.GameOverInitiated` Outcome)
  (`GameplayStatics.SetGamePaused` true))

(fn `GetExposureCompensation`
  (params (Brightness :type "Float (double-precision)"))
  (returns (ExposureCompensation :type "Float (double-precision)"))
  (bind __gameinstance (`self._GameInstance`))
  ;[1 1 1] Get Exposure Compensation
  (return (`KismetMathLibrary.MapRangeClamped` Brightness 0.5 1.5 (`/Game/ProjectName/Core/BP_GameInstance.MinimumExposureCompensation` __gameinstance) (`/Game/ProjectName/Core/BP_GameInstance.MaximumExposureCompensation` __gameinstance))))

(fn `GetSafeVolumeMultiplier`
  (params (Volume :type "Float (double-precision)"))
  (returns (SafeVolumeMultiplier :type "Float (double-precision)"))
  ;[1 1 1] Get Safe Volume Multiplier
  (if (`KismetMathLibrary.NearlyEqual_FloatFloat` Volume)
    (return (`/Game/ProjectName/Core/BP_GameInstance.MinimumSafeVolumeMultiplier` (`self._GameInstance`)))
    (else
      (return (`local.Volume`)))))

(fn `OnActiveEnemiesChanged`
  (params (ActiveEnemies :type Integer))
  ;[1 1 1] Active Enemies Changed
  (if (<= ActiveEnemies 0)
    (`self.GameOver` "NewEnumerator0")))

(fn `OnBrightnessValueChanged`
  (params (Value :type "Float (double-precision)"))
  ;[1 1 1] Brightness Value Changed
  (`self.SetBrightness` Value))

(fn `OnMusicVolumeControlChanged`
  (params (Volume :type "Float (double-precision)") (IsMuted :type Boolean))
  ;[1 1 1] Music Volume Control Changed
  (`AudioComponent.SetVolumeMultiplier` (`self.AudioMusic`) (`self.GetSafeVolumeMultiplier` (select `bool` IsMuted :`false` Volume))))

(fn `OnPlayerControllerInitialised`
  ;[1 1 1] Player Controller Initialised
  (`/Game/ProjectName/Core/Characters/Player/BP_PlayerController.InitialiseForGame` (`self._PlayerController`)))

(fn `OnPlayerPauseGameToggled`
  ;[1 1 1] Player Pause Game Toggled
  (`self.TogglePauseGame`))

(fn `OnThreatChanged`
  (params (Value :type "Float (double-precision)"))
  ;[1 1 1] Event Handler
  (if (>= Value (`/Game/ProjectName/Core/BP_GameInstance.MaximumThreatThreshold` (`self._GameInstance`)))
    (`self.GameOver` "NewEnumerator1")))

(fn `PlayMusic`
  ;[1 1 1] Play Music
  (`AudioComponent.SetSound` (`self.AudioMusic`) (`/Game/ProjectName/Core/BP_GameInstance.MusicGame` (`self._GameInstance`)))
  (`AudioComponent.Play` (`self.AudioMusic`) 0.0))

(fn `SetBrightness`
  (params (Brightness :type "Float (double-precision)"))
  ;[1 1 1] Set Brightness
  (set `PostProcessVolume.Settings` (make `PostProcessSettings` :`AutoExposureBias` (`self.GetExposureCompensation` Brightness)) (`self._PostProcessVolume`)))

(fn `SetReferences`
  ;[1 1 1] Set References
  (bind _asbp_game_instance (cast `/Game/ProjectName/Core/BP_GameInstance` (`GameplayStatics.GetGameInstance`)))
  (set `self._GameInstance` _asbp_game_instance)
  (bind _asbp_game_state (cast `/Game/ProjectName/Core/BP_GameState` (`GameplayStatics.GetGameState`)))
  (set `self._GameState` _asbp_game_state)
  (bind _asbp_player_controller (cast `/Game/ProjectName/Core/Characters/Player/BP_PlayerController` (`GameplayStatics.GetPlayerController` 0)))
  (set `self._PlayerController` _asbp_player_controller)
  (bind _outactors (`GameplayStatics.GetAllActorsOfClass` "/Script/Engine.PostProcessVolume"))
  (set `self._PostProcessVolume` (`|GetArrayItem` _outactors)))

(fn `TogglePauseGame`
  (bind _returnvalue (`GameplayStatics.IsGamePaused`))
  ;[1 1 1] Toggle Pause Game
  (`GameplayStatics.SetGamePaused` (select `bool` _returnvalue :`false` true))
  (`self.GamePauseToggled` _returnvalue))

(fn `UserConstructionScript`)