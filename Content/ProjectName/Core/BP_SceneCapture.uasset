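; BP_SceneCapture is a scene capture actor whose 2D capture component stays off until game over is initiated.
; On BeginPlay it deactivates and hides the component, caches BP_GameMode and binds to its GameOverInitiated event.
; When that event fires, it activates and shows the capture component, without using the outcome or game duration it receives.
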(event `self.ReceiveBeginPlay`
  ;[1 1 1] Initialise
  (`ActorComponent.Deactivate` (`self.CaptureComponent2D`))
  (`SceneComponent.SetVisibility` (`self.CaptureComponent2D`) false false)
  (`self.SetReferences`)
  (`self.BindToEvents`))

(fn `BindToEvents`
  ;[1 1 1] Bind to Events
  (add `/Game/ProjectName/Core/GameModes/BP_GameMode.GameOverInitiated` (`self._GameMode`) (`|CreateDelegate` :!event `OnGameOverInitiated`)))

(fn `OnGameOverInitiated`
  (params (Outcome :type "/Game/ProjectName/Core/Enums/EGameOverOutcome Enum" :default "NewEnumerator2") (GameDuration :type "Float (double-precision)"))
  ;[1 1 1] Game Over Initiated
  (`ActorComponent.Activate` (`self.CaptureComponent2D`) false)
  (`SceneComponent.SetVisibility` (`self.CaptureComponent2D`) true false))

(fn `SetReferences`
  ;[1 1 1] Set References
  (bind _asbp_game_mode (cast `/Game/ProjectName/Core/GameModes/BP_GameMode` (`GameplayStatics.GetGameMode`)))
  (set `self._GameMode` _asbp_game_mode))

(fn `UserConstructionScript`)