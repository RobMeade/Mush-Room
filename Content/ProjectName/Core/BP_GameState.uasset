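; Game state for a mushroom game that tracks active enemies, total threat and end-of-game player metrics.
; A looping timer waits for play to begin, then caches the game mode, spawners and player, binds to their events and broadcasts initialisation.
; Handlers update counts, threat and per-type destroyed, thrown and dropped mushroom metrics, broadcasting key changes.
; On game over it records outcome, duration and accuracy (destroyed over thrown plus dropped), then signals finalisation.
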(event `self.ReceiveBeginPlay`
  ;[1 1 1] Initialise
  (bind _returnvalue (`KismetSystemLibrary.K2_SetTimer` null "CanSetReferences" 0.1 true))
  (set `self._HasBegunPlayTimer` _returnvalue))

(fn `BindToEvents`
  (locals (EnemySpawner :type "/Game/ProjectName/Core/BP_MushroomSpawner Object Reference"))
  ;[1 1 1] Bind to Events
  (add `/Game/ProjectName/Core/GameModes/BP_GameMode.GameOverInitiated` (`self._GameMode`) (`|CreateDelegate` :!event `OnGameOverInitiated`))
  (for _array_element (`self._EnemySpawners`)
    (bind _output_get (set `local.EnemySpawner` _array_element))
    (add `/Game/ProjectName/Core/BP_MushroomSpawner.EnemySpawned` _output_get (`|CreateDelegate` :!event `OnEnemySpawned`))
    (add `/Game/ProjectName/Core/BP_MushroomSpawner.EnemyDestroyed` (`local.EnemySpawner`) (`|CreateDelegate` :!event `OnEnemyDestroyed`))
    (add `/Game/ProjectName/Core/Characters/Player/BP_FirstPersonCharacter.PlayerThrewObject` (`self._PlayerCharacter`) (`|CreateDelegate` :!event `OnPlayerThrewObject`))
    (add `/Game/ProjectName/Core/Characters/Player/BP_FirstPersonCharacter.PlayerDroppedObject` (`self._PlayerCharacter`) (`|CreateDelegate` :!event `OnPlayerDroppedObject`))))

(fn `CanSetReferences`
  ;[1 1 1] Can Set References?
  (if (`self.HasBegunPlay`)
    (`KismetSystemLibrary.K2_ClearAndInvalidateTimerHandle` (`self._HasBegunPlayTimer`))
    (`self.SetReferences`)
    (`self.BindToEvents`)
    (`self.Initialised`)))

(fn `GetThreat`
  (returns (Threat :type "Float (double-precision)"))
  ;[1 1 1] Get Threat
  (return (`self._Threat`)))

(fn `IncrementGameMetricDestroyedMushroom`
  (params (MushroomType :type "Object Class Reference"))
  (bind (__gamemetrics_gameduration __gamemetrics_bluemushroomdestroyed) (break `/Game/ProjectName/Core/Structures/SGameMetrics` (`self._GameMetrics`)))
  (bind (__gamemetrics_gameduration_2 __gamemetrics_bluemushroomdestroyed_2 __gamemetrics_greenmushroomdestroyed) (break `/Game/ProjectName/Core/Structures/SGameMetrics` (`self._GameMetrics`)))
  (bind (__gamemetrics_gameduration_3 __gamemetrics_bluemushroomdestroyed_3 __gamemetrics_greenmushroomdestroyed_2 __gamemetrics_redmushroomsdestroyed) (break `/Game/ProjectName/Core/Structures/SGameMetrics` (`self._GameMetrics`)))
  ;[1 1 1] Increment Game Metric - Destroyed Mushroom
  (`|ExecutionSequence`
    (:`then_0`
      (if (== (`local.MushroomType`) "/Game/ProjectName/Characters/NPC/Mushroom/BP_Mushroom_01.BP_Mushroom_01_C")
        (bind _result (`/Engine/EditorBlueprintResources/StandardMacros.IncrementInt` __gamemetrics_greenmushroomdestroyed)
          (:`  `
            (bind _structout (setmembers `/Game/ProjectName/Core/Structures/SGameMetrics` :`StructRef` (`self._GameMetrics`) :`GreenMushroomDestroyed` _result))
            (`self.GameMetricsChanged` _structout)))))
    (:`then_1`
      (if (== (`local.MushroomType`) "/Game/ProjectName/Characters/NPC/Mushroom/BP_Mushroom_02.BP_Mushroom_02_C")
        (bind _result_2 (`/Engine/EditorBlueprintResources/StandardMacros.IncrementInt` __gamemetrics_redmushroomsdestroyed)
          (:`  `
            (bind _structout_2 (setmembers `/Game/ProjectName/Core/Structures/SGameMetrics` :`StructRef` (`self._GameMetrics`) :`RedMushroomsDestroyed` _result_2))
            (`self.GameMetricsChanged` _structout_2)))))
    (:`then_2`
      (if (== (`local.MushroomType`) "/Game/ProjectName/Characters/NPC/Mushroom/BP_Mushroom_03.BP_Mushroom_03_C")
        (bind _result_3 (`/Engine/EditorBlueprintResources/StandardMacros.IncrementInt` __gamemetrics_bluemushroomdestroyed)
          (:`  `
            (bind _structout_3 (setmembers `/Game/ProjectName/Core/Structures/SGameMetrics` :`StructRef` (`self._GameMetrics`) :`BlueMushroomDestroyed` _result_3))
            (`self.GameMetricsChanged` _structout_3)))))))

(fn `IncrementGameMetricPlayerActionDropMushroom`
  (bind (__gamemetrics_gameduration __gamemetrics_bluemushroomdestroyed __gamemetrics_greenmushroomdestroyed __gamemetrics_redmushroomsdestroyed __gamemetrics_playeractionthrowmushroom __gamemetrics_playeractiondropmushroom) (break `/Game/ProjectName/Core/Structures/SGameMetrics` (`self._GameMetrics`)))
  ;[1 1 1] Increment Game Metric - Player Action Drop Mushroom
  (bind _result (`/Engine/EditorBlueprintResources/StandardMacros.IncrementInt` __gamemetrics_playeractiondropmushroom)
    (:`  `
      (setmembers `/Game/ProjectName/Core/Structures/SGameMetrics` :`StructRef` (`self._GameMetrics`) :`PlayerActionDropMushroom` _result))))

(fn `IncrementGameMetricPlayerActionThrowMushroom`
  (bind (__gamemetrics_gameduration __gamemetrics_bluemushroomdestroyed __gamemetrics_greenmushroomdestroyed __gamemetrics_redmushroomsdestroyed __gamemetrics_playeractionthrowmushroom) (break `/Game/ProjectName/Core/Structures/SGameMetrics` (`self._GameMetrics`)))
  ;[1 1 1] Increment Game Metric - Player Action Throw Mushroom
  (bind _result (`/Engine/EditorBlueprintResources/StandardMacros.IncrementInt` __gamemetrics_playeractionthrowmushroom)
    (:`  `
      (setmembers `/Game/ProjectName/Core/Structures/SGameMetrics` :`StructRef` (`self._GameMetrics`) :`PlayerActionThrowMushroom` _result))))

(fn `OnEnemyDestroyed`
  (params (MushroomType :type "Object Class Reference"))
  ;[1 1 1] Enemy Destroyed
  (`self.IncrementGameMetricDestroyedMushroom` MushroomType)
  (bind _result (`/Engine/EditorBlueprintResources/StandardMacros.DecrementInt` (`self._ActiveEnemies`))
    (:`  `
      (`self.ActiveEnemiesChanged` _result))))

(fn `OnEnemySpawned`
  (params (Enemy :type "/Game/ProjectName/Core/Characters/NPC/BP_MushroomBase Object Reference"))
  ;[1 1 1] Enemy Spawned
  (`/Engine/EditorBlueprintResources/StandardMacros.IncrementInt` (`self._ActiveEnemies`)
    (:`  `
      (add `/Game/ProjectName/Core/Characters/NPC/BP_MushroomBase.ThreatChanged` (`local.Enemy`) (`|CreateDelegate` :!event `OnEnemyThreatChanged`))
      (if (not (`self._FirstEnemySpawned`))
        (set `self._FirstEnemySpawned` true)
        (`self.FirstEnemySpawned`)))))

(fn `OnEnemyThreatChanged`
  (params (Value :type "Float (double-precision)"))
  ;[1 1 1] Event Handler
  (bind _output_get (set `self._Threat` (+ (`self._Threat`) Value)))
  (`self.ThreatChanged` _output_get))

(fn `OnGameOverInitiated`
  (params (Outcome :type "/Game/ProjectName/Core/Enums/EGameOverOutcome Enum" :default "NewEnumerator0") (GameDuration :type "Float (double-precision)"))
  ;[1 1 1] Game Over Initiated
  (set `self._Outcome` Outcome)
  (`self.SetGameMetricGameDuration` GameDuration)
  (`self.SetGameMetricPlayerAccuracy`)
  (`self.GameOverFinalised`))

(fn `OnPlayerDroppedObject`
  (params (ObjectType :type "Object Class Reference"))
  ;[1 1 1] Player Dropped Object
  (if (`KismetMathLibrary.ClassIsChildOf` ObjectType "/Game/ProjectName/Core/Characters/NPC/BP_MushroomBase.BP_MushroomBase_C")
    (`self.IncrementGameMetricPlayerActionDropMushroom`)))

(fn `OnPlayerThrewObject`
  (params (ObjectType :type "Object Class Reference"))
  ;[1 1 1] Player Threw Object
  (if (`KismetMathLibrary.ClassIsChildOf` ObjectType "/Game/ProjectName/Core/Characters/NPC/BP_MushroomBase.BP_MushroomBase_C")
    (`self.IncrementGameMetricPlayerActionThrowMushroom`)))

(fn `SetGameMetricGameDuration`
  (params (GameDuration :type "Float (double-precision)"))
  ;[1 1 1] Set Game Metric - Game Duration
  (setmembers `/Game/ProjectName/Core/Structures/SGameMetrics` :`StructRef` (`self._GameMetrics`) :`GameDuration` GameDuration))

(fn `SetGameMetricPlayerAccuracy`
  (bind (__gamemetrics_gameduration __gamemetrics_bluemushroomdestroyed __gamemetrics_greenmushroomdestroyed __gamemetrics_redmushroomsdestroyed __gamemetrics_playeractionthrowmushroom __gamemetrics_playeractiondropmushroom) (break `/Game/ProjectName/Core/Structures/SGameMetrics` (`self._GameMetrics`)))
  ;[1 1 1] Set Game Metric - Player Accuracy
  (setmembers `/Game/ProjectName/Core/Structures/SGameMetrics` :`StructRef` (`self._GameMetrics`) :`PlayerAccuracy` (/ (`KismetMathLibrary.Conv_IntToDouble` (+ __gamemetrics_bluemushroomdestroyed __gamemetrics_greenmushroomdestroyed __gamemetrics_redmushroomsdestroyed)) (`KismetMathLibrary.Conv_IntToDouble` (+ __gamemetrics_playeractionthrowmushroom __gamemetrics_playeractiondropmushroom)))))

(fn `SetReferences`
  ;[1 1 1] Set References
  (bind _asbp_game_mode (cast `/Game/ProjectName/Core/GameModes/BP_GameMode` (`GameplayStatics.GetGameMode`)))
  (set `self._GameMode` _asbp_game_mode)
  (bind _outactors (`GameplayStatics.GetAllActorsOfClass` "/Game/ProjectName/Core/BP_MushroomSpawner.BP_MushroomSpawner_C"))
  (set `self._EnemySpawners` _outactors)
  (bind _asbp_first_person_character (cast `/Game/ProjectName/Core/Characters/Player/BP_FirstPersonCharacter` (`GameplayStatics.GetPlayerCharacter` 0)))
  (set `self._PlayerCharacter` _asbp_first_person_character))

(fn `UserConstructionScript`)