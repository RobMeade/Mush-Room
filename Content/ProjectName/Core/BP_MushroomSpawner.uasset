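; BP_MushroomSpawner is a placeable volume that spawns fixed or random mushroom enemies once the game mode signals initialisation.
; Spawn mode uses re-armed random-delay timers under a concurrent cap; Burst mode spawns random-sized groups, optionally looping.
; Random points in the box are line-traced downward to align enemies to the surface.
; Enemy self-destruct events update active counts, while total caps, an optional lifetime and game over halt spawning.
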(event `self.ReceiveBeginPlay`
  ;[1 1 1] Initialise
  (`self.SetReferences`)
  (`self.BindToEvents`))

(fn `BindToEvents`
  ;[1 1 1] Bind to Events
  (add `/Game/ProjectName/Core/GameModes/BP_GameMode.GameInitialised` (`self._GameMode`) (`|CreateDelegate` :!event `OnGameInitialised`))
  (add `/Game/ProjectName/Core/GameModes/BP_GameMode.GameOverInitiated` (`self._GameMode`) (`|CreateDelegate` :!event `OnGameOverInitiated`)))

(fn `Burst`
  ;[1 1 1] Burst
  (for _ (range 1 (+ (`self._BurstCount`) 1))
    (if (and (`self._CanBurst`) (not (`self._HasExpired`)))
      (`self.Spawn`))))

(fn `ClearTimer`
  (params (TimerHandle :type "TimerHandle Structure"))
  ;[1 1 1] Clear Timer
  (if (`KismetSystemLibrary.K2_TimerExistsHandle` TimerHandle)
    (`KismetSystemLibrary.K2_ClearAndInvalidateTimerHandle` (`local.TimerHandle`))))

(fn `ConfigureLifetime`
  ;[1 1 1] Configure Lifetime
  (`self.SetLifetimeTimer`))

(fn `ConfigureMode`
  ;[1 1 1] Configure Mode
  (switch `/Game/ProjectName/Core/Enums/EEnemySpawnerMode` (`self.Mode`)
    (:`NewEnumerator0`
      (`self.ConfigureModeSpawn`))
    (:`NewEnumerator1`
      (`self.ConfigureModeBurst`))))

(fn `ConfigureModeBurst`
  ;[1 1 1] Configure Burst Mode
  (if (> (`self.MinimumBurstCount`) 0)
    (`self.SetRandomBurstCount`)
    (`self.SetRandomBurstDelay`)
    (`self.SetBurstTimer` (`self.InitialBurstDelay`) (`self.GetSafeTimerDelayTime` 0.0))))

(fn `ConfigureModeSpawn`
  ;[1 1 1] Configure Spawn Mode
  (if (> (`self.MaximumConcurrentEnemies`) 0)
    (`self.SetSpawnTimer` (`self.InitialSpawnDelay`) (`self.GetSafeTimerDelayTime` 0.0))))

(fn `ConfigureRandomOnceEnemyToSpawn`
  ;[1 1 1] Configure Random Once Enemy to Spawn
  (if (`|EnumEquality` (`self.SpawnEnemy`) "NewEnumerator3")
    (set `self._RandomOnceEnemyToSpawn` (`self.GetRandomEnemy`))))

(fn `GetEnemyToSpawn`
  (returns (Enemy :type "/Game/ProjectName/Core/Characters/NPC/BP_MushroomBase Class Reference"))
  ;[1 1 1] Get Enemy to Spawn
  (return (select `/Game/ProjectName/Core/Enums/EEnemySpawnerSpawnOption` (`self.SpawnEnemy`) :`NewEnumerator3` (`self._RandomOnceEnemyToSpawn`) :`NewEnumerator4` (`self.GetRandomEnemy`) :`NewEnumerator2` "/Game/ProjectName/Characters/NPC/Mushroom/BP_Mushroom_03.BP_Mushroom_03_C" :`NewEnumerator0` "/Game/ProjectName/Characters/NPC/Mushroom/BP_Mushroom_01.BP_Mushroom_01_C" :`NewEnumerator1` "/Game/ProjectName/Characters/NPC/Mushroom/BP_Mushroom_02.BP_Mushroom_02_C")))

(fn `GetRandomEnemy`
  (returns (Enemy :type "/Game/ProjectName/Core/Characters/NPC/BP_MushroomBase Class Reference"))
  ;[1 1 1] Get Random Enemy
  (return (select `int` (`KismetMathLibrary.RandomIntegerInRange` 0 2) :`0` "/Game/ProjectName/Characters/NPC/Mushroom/BP_Mushroom_01.BP_Mushroom_01_C" :`1` "/Game/ProjectName/Characters/NPC/Mushroom/BP_Mushroom_02.BP_Mushroom_02_C" :`2` "/Game/ProjectName/Characters/NPC/Mushroom/BP_Mushroom_03.BP_Mushroom_03_C" :!type "/Game/ProjectName/Core/Characters/NPC/BP_MushroomBase Class Reference")))

(fn `GetRandomSpawnLocation`
  (returns (SpawnLocation :type "Vector Structure"))
  (bind (_returnvalue_x _returnvalue_y _returnvalue_z) (`KismetMathLibrary.BreakVector` (`self.K2_GetActorLocation`)))
  (bind _spawnvolume (`self.SpawnVolume`))
  ;[1 1 1] Get Random Spawn Location
  (return (`KismetMathLibrary.MakeVector` (.x (`KismetMathLibrary.TransformLocation` (`self.GetTransform`) (`KismetMathLibrary.RandomPointInBoundingBox` (`SceneComponent.RelativeLocation` _spawnvolume) (`BoxComponent.BoxExtent` _spawnvolume)))) (.y (`KismetMathLibrary.TransformLocation` (`self.GetTransform`) (`KismetMathLibrary.RandomPointInBoundingBox` (`SceneComponent.RelativeLocation` _spawnvolume) (`BoxComponent.BoxExtent` _spawnvolume)))) (+ _returnvalue_z (`self.SpawnVolumeHeight`)))))

(fn `GetSafeTimerDelayTime`
  (params (Time :type "Float (double-precision)"))
  (returns (SafeTimerDelayTime :type "Float (double-precision)"))
  ;[1 1 1] Get Safe Timer Delay Time
  (if (`KismetMathLibrary.NearlyEqual_FloatFloat` Time)
    (return 0.001)
    (else
      (return (`local.Time`)))))

(fn `Initialise`
  ;[1 1 1] Initialise
  (`self.ConfigureLifetime`)
  (`self.ConfigureMode`)
  (`self.ConfigureRandomOnceEnemyToSpawn`))

(fn `OnBurst`
  ;[1 1 1] Burst (multiple) enemies
  (`self.ClearTimer` (`self._BurstTimerHandle`))
  (if (and (`self._CanBurst`) (not (`self._HasExpired`)))
    (`self.Burst`))
  (if (`self.BurstLoop`)
    (`self.SetRandomBurstCount`)
    (`self.SetRandomBurstDelay`)
    (`self.SetBurstTimer` 0.0 (`self._BurstDelay`))))

(fn `OnEnemyDestroyed`
  (params (MushroomType :type "Object Class Reference"))
  ;[1 1 1] Enemy Destroyed
  (`/Engine/EditorBlueprintResources/StandardMacros.DecrementInt` (`self._ActiveEnemies`)
    (:`  `
      (`self.SetCanSpawn`)
      (`self.EnemyDestroyed` (`local.MushroomType`)))))

(fn `OnGameInitialised`
  ;[1 1 1] Initialise
  (`self.Initialise`))

(fn `OnGameOverInitiated`
  (params (Outcome :type "/Game/ProjectName/Core/Enums/EGameOverOutcome Enum" :default "NewEnumerator0") (GameDuration :type "Float (double-precision)"))
  ;[1 1 1] Game Over Initiated
  (`self.ClearTimer` (`self._SpawnTimerHandle`))
  (`self.ClearTimer` (`self._BurstTimerHandle`))
  (set `self._CanSpawn` false)
  (set `self._CanBurst` false))

(fn `OnLifetimeExpired`
  ;[1 1 1] Lifetime Expired
  (`self.ClearTimer` (`self._LifetimeTimerHandle`))
  (set `self._HasExpired` true))

(fn `OnSpawn`
  ;[1 1 1] Spawn an Enemy
  (`self.ClearTimer` (`self._SpawnTimerHandle`))
  (if (not (`self._HasExpired`))
    (`self.SetRandomSpawnDelay`)
    (`self.SetSpawnTimer` 0.0 (`self._SpawnDelay`))
    (if (`self._CanSpawn`)
      (`self.Spawn`))))

(fn `SetBurstTimer`
  (params (InitialBurstDelay :type "Float (double-precision)") (LoopDelay :type "Float (double-precision)"))
  (locals (Time :type "Float (double-precision)"))
  ;[1 1 1] Set Burst Timer
  (if (`KismetMathLibrary.NearlyEqual_FloatFloat` InitialBurstDelay)
    (set `local.Time` (`local.LoopDelay`))
    (else
      (set `local.Time` (`self.GetSafeTimerDelayTime` 0.0))))
  (bind _returnvalue (`KismetSystemLibrary.K2_SetTimerDelegate` (`|CreateDelegate` :!event `OnBurst`) (`local.Time`) false (`local.InitialBurstDelay`)))
  (set `self._BurstTimerHandle` _returnvalue))

(fn `SetCanBurst`
  ;[1 1 1] Set Can Burst
  (if (> (`self.MaximumSpawnCount`) 0)
    (set `self._CanBurst` (< (`self._SpawnedEnemies`) (`self.MaximumSpawnCount`)))
    (else
      (set `self._CanBurst` true))))

(fn `SetCanSpawn`
  ;[1 1 1] Set Can Spawn
  (if (> (`self.MaximumSpawnCount`) 0)
    (set `self._CanSpawn` (and (< (`self._SpawnedEnemies`) (`self.MaximumSpawnCount`)) (< (`self._ActiveEnemies`) (`self.MaximumConcurrentEnemies`))))
    (else
      (set `self._CanSpawn` (< (`self._ActiveEnemies`) (`self.MaximumConcurrentEnemies`))))))

(fn `SetLifetimeTimer`
  ;[1 1 1] Set Lifetime Timer
  (if (> (`self.MaximumLifeTime`) 0.0)
    (bind _returnvalue (`KismetSystemLibrary.K2_SetTimerDelegate` (`|CreateDelegate` :!event `OnLifetimeExpired`) (`self.MaximumLifeTime`)))
    (set `self._LifetimeTimerHandle` _returnvalue)))

(fn `SetRandomBurstCount`
  ;[1 1 1] Set Random Burst Count
  (set `self._BurstCount` (`KismetMathLibrary.RandomIntegerInRange` (`self.MinimumBurstCount`) (`self.MaximumBurstCount`))))

(fn `SetRandomBurstDelay`
  ;[1 1 1] Set Random Burst Delay
  (set `self._BurstDelay` (`KismetMathLibrary.RandomFloatInRange` (`self.MinimumBurstLoopDelay`) (`self.MaximumBurstLoopDelay`))))

(fn `SetRandomSpawnDelay`
  ;[1 1 1] Set Random Spawn Delay
  (set `self._SpawnDelay` (`KismetMathLibrary.RandomFloatInRange` (`self.MinimumSpawnDelay`) (`self.MaximumSpawnDelay`))))

(fn `SetReferences`
  ;[1 1 1] Set References
  (bind _asbp_game_instance (cast `/Game/ProjectName/Core/BP_GameInstance` (`GameplayStatics.GetGameInstance`)))
  (set `self._GameInstance` _asbp_game_instance)
  (bind _asbp_game_mode (cast `/Game/ProjectName/Core/GameModes/BP_GameMode` (`GameplayStatics.GetGameMode`)))
  (set `self._GameMode` _asbp_game_mode))

(fn `SetSpawnTimer`
  (params (InitialSpawnDelay :type "Float (double-precision)") (SpawnDelay :type "Float (double-precision)"))
  (locals (Time :type "Float (double-precision)"))
  ;[1 1 1] Set Spawn Timer
  (if (`KismetMathLibrary.NearlyEqual_FloatFloat` InitialSpawnDelay)
    (set `local.Time` (`local.SpawnDelay`))
    (else
      (set `local.Time` (`self.GetSafeTimerDelayTime` 0.0))))
  (bind _returnvalue (`KismetSystemLibrary.K2_SetTimerDelegate` (`|CreateDelegate` :!event `OnSpawn`) (`local.Time`) false (`local.InitialSpawnDelay`)))
  (set `self._SpawnTimerHandle` _returnvalue))

(fn `SetSpawnTransformBasedOnCollision`
  (params (SpawnLocation :type "Vector Structure"))
  (bind (_returnvalue_roll _returnvalue_pitch _returnvalue_yaw) (`KismetMathLibrary.BreakRotator` (`KismetMathLibrary.RandomRotator` false)))
  (bind (_spawnlocation_x _spawnlocation_y _spawnlocation_z) (`KismetMathLibrary.BreakVector` (`local.SpawnLocation`)))
  (bind (_returnvalue_roll_2 _returnvalue_pitch_2) (`KismetMathLibrary.BreakRotator` (`SceneComponent.K2_GetComponentRotation` (`self.DefaultSceneRoot`))))
  ;[1 1 1] Set Spawn Transform Based on Collision
  (bind _outhit (`KismetSystemLibrary.LineTraceSingle` SpawnLocation (`KismetMathLibrary.MakeVector` (.x SpawnLocation) (.y SpawnLocation) (- (.z SpawnLocation) (`self.SpawnVolumeHeight`))) "TraceTypeQuery1" true))
  (bind (_bblockinghit _binitialoverlap _time _distance _location _impactpoint _normal _impactnormal) (`GameplayStatics.BreakHitResult` _outhit))
  (if _bblockinghit
    (set `self._SpawnTransform` (`KismetMathLibrary.MakeTransform` _impactpoint (`KismetMathLibrary.MakeRotFromZX` _impactnormal (`SceneComponent.GetForwardVector` (`self.DefaultSceneRoot`)))))
    (else
      (set `self._SpawnTransform` (`KismetMathLibrary.MakeTransform` (`KismetMathLibrary.MakeVector` _spawnlocation_x _spawnlocation_y (- _spawnlocation_z (`self.SpawnVolumeHeight`))) (`KismetMathLibrary.MakeRotator` _returnvalue_roll_2 _returnvalue_pitch_2 _returnvalue_yaw))))))

(fn `Spawn`
  (locals (SpawnedEnemy :type "/Game/ProjectName/Core/Characters/NPC/BP_MushroomBase Object Reference"))
  ;[1 1 1] Spawn
  (`self.SetSpawnTransformBasedOnCollision` (`self.GetRandomSpawnLocation`))
  (bind _returnvalue (`|SpawnActorFromClass` (`self.GetEnemyToSpawn`) (`self._SpawnTransform`) "Undefined" "OverrideRootScale" null null))
  (bind _output_get (set `local.SpawnedEnemy` _returnvalue))
  (add `/Game/ProjectName/Core/Characters/NPC/BP_MushroomBase.SelfDestructInitiated` _output_get (`|CreateDelegate` :!event `OnEnemyDestroyed`))
  (`self.EnemySpawned` (`local.SpawnedEnemy`))
  (`/Engine/EditorBlueprintResources/StandardMacros.IncrementInt` (`self._ActiveEnemies`)
    (:`  `
      (`/Engine/EditorBlueprintResources/StandardMacros.IncrementInt` (`self._SpawnedEnemies`)
        (:`  `
          (switch `/Game/ProjectName/Core/Enums/EEnemySpawnerMode` (`self.Mode`)
            (:`NewEnumerator0`
              (`self.SetCanSpawn`))
            (:`NewEnumerator1`
              (`self.SetCanBurst`))))))))

(fn `UserConstructionScript`
  (bind (_returnvalue_roll _returnvalue_pitch _returnvalue_yaw) (`KismetMathLibrary.BreakRotator` (`self.K2_GetActorRotation`)))
  (bind _returnvalue (/ (`self.SpawnVolumeHeight`) 2.0))
  ;[1 1 1] Instantiate
  (`BoxComponent.SetBoxExtent` (`self.SpawnVolume`) (`KismetMathLibrary.MakeVector` (/ (`self.SpawnVolumeWidth`) 2.0) (/ (`self.SpawnVolumeLength`) 2.0) _returnvalue) true)
  (`SceneComponent.K2_SetRelativeLocation` (`self.SpawnVolume`) (`KismetMathLibrary.MakeVector` 0.0 0.0 _returnvalue) false false)
  (`self.K2_SetActorRotation` (`KismetMathLibrary.MakeRotator` 0.0 0.0 _returnvalue_yaw)))