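; BP_MushroomBase is the base mushroom enemy NPC, which can be grabbed, released, highlighted and destroyed.
; Grabbing sets its state, disables shadow casting and starts a randomly timed cycle of random held animation states.
; EnemyThreatComponent changes are relayed through its own event, and threat emission stops at game over.
; GameInstance supplies sounds and SFX volume preferences, while highlighting uses a material scalar parameter.
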(event `self.ReceiveBeginPlay`
  ;[1 1 1] Initialise
  (`self.SetReferences`)
  (`self.BindToEvents`)
  (`self.BindToComponentEvents`)
  (`self.SetEnemyAudioSFX`)
  (`KismetSystemLibrary.Delay` 0.2)
  (`self.Initialise`)
  (set `self.State` "NewEnumerator1")
  (`self.PlaySpawnSFX`))

(event `/Game/ProjectName/Core/Interfaces/BPI_Grabbable.Grab`
  ;[1 1 1] Grabbable
  (set `self.State` "NewEnumerator2")
  (`self.OnUpdateHeldAnimationState`)
  (`self.PlayPickUpSFX`)
  (`PrimitiveComponent.SetCastShadow` (`self.SkeletalMesh`) false))

(event `/Game/ProjectName/Core/Interfaces/BPI_Grabbable.Highlight`
  (params (Enabled :type Boolean))
  ;[1 1 1] Highlight
  (`self.SetHighlightingState` Enabled))

(event `/Game/ProjectName/Core/Interfaces/BPI_Grabbable.Release`
  (params (Thrown :type Boolean))
  ;[1 1 1] Grabbable
  (set `self.State` "NewEnumerator0")
  (`self.OnUpdateHeldAnimationState`)
  (`PrimitiveComponent.SetCastShadow` (`self.SkeletalMesh`) true))

(event `/Game/ProjectName/Core/Interfaces/BPI_Destructible.Destroy`
  ;[1 1 1] Self Destruct
  (`self.SelfDestruct`))

(fn `BindToComponentEvents`
  ;[1 1 1] Bind to Component Events
  (add `/Game/ProjectName/Core/Characters/NPC/BP_MushroomThreat_Component.ThreatChanged` (`self.EnemyThreatComponent`) (`|CreateDelegate` :!event `OnThreatChanged`)))

(fn `BindToEvents`
  ;[1 1 1] Bind to Events
  (add `/Game/ProjectName/Core/BP_GameInstance.PlayerPreferencesChanged` (`self._GameInstance`) (`|CreateDelegate` :!event `OnPlayerPreferencesChanged`))
  (add `/Game/ProjectName/Core/GameModes/BP_GameMode.GameOverInitiated` (`self._GameMode`) (`|CreateDelegate` :!event `OnGameOverInitiated`)))

(fn `GetHeldAnimationStateDuration`
  (returns (Duration :type "Float (double-precision)"))
  (bind __gameinstance (`self._GameInstance`))
  ;[1 1 1] Get Held Animation State Duration
  (return (`KismetMathLibrary.RandomFloatInRange` (`/Game/ProjectName/Core/BP_GameInstance.MushroomMinimumHeldAnimationStateDuration` __gameinstance) (`/Game/ProjectName/Core/BP_GameInstance.MushroomMaximumHeldAnimationStateDuration` __gameinstance))))

(fn `GetSafeVolumeMultiplier`
  (params (Volume :type "Float (double-precision)"))
  (returns (SafeVolumeMultiplier :type "Float (double-precision)"))
  ;[1 1 1] Get Safe Volume Multiplier
  (if (`KismetMathLibrary.NearlyEqual_FloatFloat` Volume)
    (return (`/Game/ProjectName/Core/BP_GameInstance.MinimumSafeVolumeMultiplier` (`self._GameInstance`)))
    (else
      (return (`local.Volume`)))))

(fn `Initialise`
  ;[1 1 1] Initialise
  (`/Game/ProjectName/Core/Characters/NPC/BP_MushroomThreat_Component.Initialise` (`self.EnemyThreatComponent`)))

(fn `OnGameOverInitiated`
  (params (Outcome :type "/Game/ProjectName/Core/Enums/EGameOverOutcome Enum" :default "NewEnumerator0") (GameDuration :type "Float (double-precision)"))
  ;[1 1 1] Event Handler
  (`/Game/ProjectName/Core/Characters/NPC/BP_MushroomThreat_Component.StopEmittingThreat` (`self.EnemyThreatComponent`)))

(fn `OnPlayerPreferencesChanged`
  ;[1 1 1] Player Preferences Updated
  (`self.SetEnemyAudioVolumeMultiplier`))

(fn `OnThreatChanged`
  (params (Value :type "Float (double-precision)"))
  ;[1 1 1] Raise Event
  (`self.ThreatChanged` Value))

(fn `OnUpdateHeldAnimationState`
  ;[1 1 1] Update Held Animation State
  (`KismetSystemLibrary.K2_ClearAndInvalidateTimerHandle` (`self._HeldAnimationStateTimerHandle`))
  (if (`|EnumEquality` (`self.State`) "NewEnumerator2")
    (`self.SetRandomHeldAnimationState`)
    (`self.SetHeldAnimationStateDuration`)
    (`self.SetHeldAnimationStateUpdateTimer`)))

(fn `PlayDestroyedSFX`
  (bind (_audiopreferences_musicvolume _audiopreferences_musicismuted _audiopreferences_sfxvolume _audiopreferences_sfxismuted) (break `/Game/ProjectName/Core/Structures/PlayerPreferences/SPlayerPreferencesAudio` (`/Game/ProjectName/Core/BP_GameInstance.GetPlayerPreferencesAudio` (`self._GameInstance`))))
  ;[1 1 1] Play Destroyed SFX
  (`GameplayStatics.SpawnSoundAtLocation` (`/Game/ProjectName/Core/BP_GameInstance.EnemyDestroyedSFX` (`self._GameInstance`)) (`self.K2_GetActorLocation`) (`self.K2_GetActorRotation`) (`self.GetSafeVolumeMultiplier` (select `bool` _audiopreferences_sfxismuted :`false` _audiopreferences_sfxvolume)) 1.0 0.0 (`/Game/ProjectName/Core/BP_GameInstance.EnemyDestroyedAttenuation` (`self._GameInstance`)) null))

(fn `PlayPickUpSFX`
  ;[1 1 1] Play Pick Up SFX
  (if (not (`AudioComponent.IsPlaying` (`self.AudioPickUp`)))
    (`AudioComponent.Play` (`self.AudioPickUp`) 0.0)))

(fn `PlaySpawnSFX`
  ;[1 1 1] Play Spawn SFX
  (if (not (`AudioComponent.IsPlaying` (`self.AudioSpawn`)))
    (`AudioComponent.Play` (`self.AudioSpawn`) 0.0)))

(fn `SelfDestruct`
  ;[1 1 1] Self Destruct
  (`self.SelfDestructInitiated` (`GameplayStatics.GetObjectClass` self))
  (`self.PlayDestroyedSFX`)
  (`self.UnbindEvents`)
  (`self.K2_DestroyActor`))

(fn `SetEnemyAudioSFX`
  ;[1 1 1] Set Enemy Audio SFX
  (`AudioComponent.SetSound` (`self.AudioSpawn`) (`/Game/ProjectName/Core/BP_GameInstance.EnemySpawnSFX` (`self._GameInstance`)))
  (set `AudioComponent.AttenuationSettings` (`/Game/ProjectName/Core/BP_GameInstance.EnemySpawnAttenuation` (`self._GameInstance`)) (`self.AudioSpawn`))
  (`AudioComponent.SetSound` (`self.AudioPickUp`) (`/Game/ProjectName/Core/BP_GameInstance.EnemyPickUpSFX` (`self._GameInstance`)))
  (set `AudioComponent.AttenuationSettings` (`/Game/ProjectName/Core/BP_GameInstance.EnemyPickUpAttenuation` (`self._GameInstance`)) (`self.AudioPickUp`))
  (`self.SetEnemyAudioVolumeMultiplier`))

(fn `SetEnemyAudioVolumeMultiplier`
  (bind (_audiopreferences_musicvolume _audiopreferences_musicismuted _audiopreferences_sfxvolume _audiopreferences_sfxismuted) (break `/Game/ProjectName/Core/Structures/PlayerPreferences/SPlayerPreferencesAudio` (`/Game/ProjectName/Core/BP_GameInstance.GetPlayerPreferencesAudio` (`self._GameInstance`))))
  (bind _safevolumemultiplier (`self.GetSafeVolumeMultiplier` (select `bool` _audiopreferences_sfxismuted :`false` _audiopreferences_sfxvolume)))
  ;[1 1 1] Set Enemy Audio Volume Multipler
  (`AudioComponent.SetVolumeMultiplier` (`self.AudioSpawn`) _safevolumemultiplier)
  (`AudioComponent.SetVolumeMultiplier` (`self.AudioPickUp`) _safevolumemultiplier))

(fn `SetHeldAnimationStateDuration`
  ;[1 1 1] Set Held Animation State Duration
  (set `self._HeldAnimationStateDuration` (`self.GetHeldAnimationStateDuration`)))

(fn `SetHeldAnimationStateUpdateTimer`
  ;[1 1 1] Set Held Animation State Change Timer
  (bind _returnvalue (`KismetSystemLibrary.K2_SetTimerDelegate` (`|CreateDelegate` :!event `OnUpdateHeldAnimationState`) (`self._HeldAnimationStateDuration`)))
  (set `self._HeldAnimationStateTimerHandle` _returnvalue))

(fn `SetHighlightingState`
  (params (Enabled :type Boolean))
  ;[1 1 1] Set Highlighting State
  (`MeshComponent.SetScalarParameterValueOnMaterials` (`self.SkeletalMesh`) "Highlighted" (select `bool` Enabled :`true` 1.0 :!type "Float (single-precision)")))

(fn `SetRandomHeldAnimationState`
  ;[1 1 1] Set Random Held Animation State
  (set `self.HeldAnimationState` (cast `/Game/ProjectName/Core/Enums/EMushroomHeldAnimationState` (`KismetMathLibrary.Conv_IntToByte` (`KismetMathLibrary.RandomIntegerInRange` 1 (- (enumcount `/Game/ProjectName/Core/Enums/EMushroomHeldAnimationState`) 1))))))

(fn `SetReferences`
  ;[1 1 1] Set References
  (bind _asbp_game_instance (cast `/Game/ProjectName/Core/BP_GameInstance` (`GameplayStatics.GetGameInstance`)))
  (set `self._GameInstance` _asbp_game_instance)
  (bind _asbp_game_mode (cast `/Game/ProjectName/Core/GameModes/BP_GameMode` (`GameplayStatics.GetGameMode`)))
  (set `self._GameMode` _asbp_game_mode))

(fn `UnbindEvents`
  ;[1 1 1] Unbind Events
  (clear `self.ThreatChanged`)
  (clear `self.SelfDestructInitiated`))

(fn `UserConstructionScript`)