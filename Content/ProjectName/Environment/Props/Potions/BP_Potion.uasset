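; Potion prop actor whose bottle shape and liquid look are set by type variables.
; The construction script looks up the static mesh from a potion type map, then applies a shared glass material to the first slot and a mapped liquid material to the second.
; A Destroy event calls SelfDestruct, which removes the actor.
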(event `/Game/ProjectName/Core/Interfaces/BPI_Destructible.Destroy`
  ;[1 1 1] Self Destruct
  (`self.SelfDestruct`))

(fn `SelfDestruct`
  ;[1 1 1] Self Destruct
  (`self.K2_DestroyActor`))

(fn `UserConstructionScript`
  ;[1 1 1] Instantiate
  (`StaticMeshComponent.SetStaticMesh` (`self.StaticMesh`) (`BlueprintMapLibrary.Map_Find` (`self._PotionType`) (`self.PotionType`)))
  (`PrimitiveComponent.SetMaterial` (`self.StaticMesh`) 0 "/Game/ProjectName/Environment/Props/Potions/M_PotionGlass.M_PotionGlass")
  (`PrimitiveComponent.SetMaterial` (`self.StaticMesh`) 1 (`BlueprintMapLibrary.Map_Find` (`self._PotionLiquidType`) (`self.LiquidType`))))