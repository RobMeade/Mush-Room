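; BP_Book is a book prop actor with a configurable cover colour and size.
; The construction script looks up a material from a colour map, assigns it to the mesh's "Cover" slot and applies the Scale value to the actor.
; A Destroy event calls SelfDestruct, which destroys the actor.
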(event `/Game/ProjectName/Core/Interfaces/BPI_Destructible.Destroy`
  ;[1 1 1] Self Destruct
  (`self.SelfDestruct`))

(fn `SelfDestruct`
  ;[1 1 1] Self Destruct
  (`self.K2_DestroyActor`))

(fn `UserConstructionScript`
  ;[1 1 1] Instantiate
  (`PrimitiveComponent.SetMaterialByName` (`self.StaticMesh`) "Cover" (`BlueprintMapLibrary.Map_Find` (`self._Colour`) (`self.Colour`)))
  (`self.SetActorScale3D` self (`self.Scale`)))