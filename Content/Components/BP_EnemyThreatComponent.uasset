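; Enemy component that tracks the threat a BP_EnemyBase owner emits, growing it over time from an initial spawn value.
; Initialise sets the starting value and per-second rate, then enables emission.
; While enabled, Tick accumulates threat and broadcasts the running total, not the frame's increment, through ThreatChanged.
; It binds to the owner's self-destruct event, whose handler stops emission and broadcasts the negated total.
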(event `self.ReceiveBeginPlay`
  ;[1 1 1] Initialise
  (`self.SetReferences`)
  (`self.BindToEvents`))

(event `self.ReceiveTick`
  (params (DeltaSeconds :type "Float (single-precision)"))
  ;[1 1 1] Increment Threat
  (if (`self.CanEmitThreat`)
    (`self.IncrementThreatEmitted` DeltaSeconds)
    (`self.ThreatChanged` (`self.ThreatEmitted`))))

(fn `BindToEvents`
  ;[1 1 1] Bind to Events
  (add `/Game/Blueprint/BP_EnemyBase.SelfDestructInitiated` (`self.Owner`) (`|CreateDelegate` :!event `OnSelfDestructInitialised`)))

(fn `IncrementThreatEmitted`
  (params (Delta :type "Float (double-precision)"))
  ;[1 1 1] Increment Threat Emitted
  (set `self.ThreatEmitted` (+ (`self.ThreatEmitted`) (* (`self.ThreatEmittedPerSecond`) Delta))))

(fn `Initialise`
  (params (ThreatEmittedOnSpawn :type "Float (double-precision)") (ThreatEmittedPerSecond :type "Float (double-precision)"))
  ;[1 1 1] Initialise
  (set `self.ThreatEmitted` ThreatEmittedOnSpawn)
  (set `self.ThreatEmittedPerSecond` ThreatEmittedPerSecond)
  (`self.StartEmittingThreat`))

(fn `OnSelfDestructInitialised`
  (locals (NewLocalVar_0 :type "Float (double-precision)"))
  ;[1 1 1] Event Handler
  (`self.StopEmittingThreat`)
  (`self.ThreatChanged` (* (`self.ThreatEmitted`) -1.0)))

(fn `SetReferences`
  ;[1 1 1] Set References
  (bind _asbp_enemy_base (cast `/Game/Blueprint/BP_EnemyBase` (`self.GetOwner`)))
  (set `self.Owner` _asbp_enemy_base))

(fn `StartEmittingThreat`
  ;[1 1 1] Start Emitting Threat
  (set `self.CanEmitThreat` true))

(fn `StopEmittingThreat`
  ;[1 1 1] Stop Emitting Threat
  (set `self.CanEmitThreat` false))